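; BP_Missile2 is a homing missile that damages what it hits and then destroys itself.
; While a homing target is flagged, Tick sweeps it straight toward MyTarget with capped acceleration and snaps its rotation to face it.
; It destroys itself if that target becomes invalid.
; Overlap applies fixed damage to any actor except BP_MissileDefence, which it ignores; a leftover BP_Meteor branch is disconnected.
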(event `self.ReceiveActorBeginOverlap`
  (params (OtherActor :type "Actor Object Reference"))
  (cast `/Game/ProjectOre/LevelElements/BP_MissileDefence` OtherActor
    (:`CastFailed`
      (`GameplayStatics.ApplyDamage` OtherActor 100.0 null self)
      (`self.K2_DestroyActor`))))

(event `self.ReceiveTick`
  (params (DeltaSeconds :type "Float (single-precision)"))
  (bind _mytarget (`self.MyTarget`))
  (bind _returnvalue (`KismetMathLibrary.GetDirectionUnitVector` (`self.K2_GetActorLocation`) (`self.K2_GetActorLocation` _mytarget)))
  (if (`self.bValidHomingTarget`)
    (`/Engine/EditorBlueprintResources/StandardMacros.IsValid` _mytarget
      (:`Is Valid`
        (`self.K2_AddActorWorldOffset` (* _returnvalue (* (`self.speed`) DeltaSeconds)) true)
        (set `self.speed` (`KismetMathLibrary.FClamp` (+ (* DeltaSeconds (`self.Acceleration`)) (`self.speed`)) 0.0 10000.0))
        (`self.K2_SetActorRotation` (`KismetMathLibrary.MakeRotFromX` _returnvalue)))
      (:`Is Not Valid`
        (`self.K2_DestroyActor`)))))

(fn `UserConstructionScript`)