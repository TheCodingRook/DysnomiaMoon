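; Player spacecraft pawn that arms itself with a gun and twin missile launchers and handles missile firing.
; BeginPlay spawns the weapons, attaches them to fighter mesh sockets and hands them to the firing and bombing components.
; DropBombBP alternates launchers via a FlipFlop, spawning missiles with sound and extra speed derived from the craft's X-axis velocity and facing.
; A timer re-enables missile fire after each shot.
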(event `self.ReceiveBeginPlay`
  (bind _returnvalue (`SceneComponent.K2_GetComponentToWorld` (`self.FighterJetMesh`)))
  ;[0.9453 1 0] Automatically equip Gun
  (bind _returnvalue_2 (`|SpawnActorFromClass` "/Game/ProjectOre/Weapons/BP_SpaceCraftGun.BP_SpaceCraftGun_C" _returnvalue "AlwaysSpawn" "OverrideRootScale" null null))
  (`/Engine/EditorBlueprintResources/StandardMacros.IsValid` _returnvalue_2
    (:`Is Valid`
      (`self.K2_AttachToComponent` _returnvalue_2 (`self.FighterJetMesh`) "GunSocket" "SnapToTarget" "SnapToTarget" "KeepRelative" true)
      (set `OreFiringComponent.EquippedWeapon` _returnvalue_2 (`self.FiringComponent`))
      ;[1 0 0.5625] Automatically equip Missile Launchers
      (bind _returnvalue_3 (`|SpawnActorFromClass` "/Game/ProjectOre/Weapons/BP_SpacecraftLauncher.BP_SpacecraftLauncher_C" _returnvalue "Undefined" "OverrideRootScale" null null))
      (`/Engine/EditorBlueprintResources/StandardMacros.IsValid` _returnvalue_3
        (:`Is Valid`
          (`self.K2_AttachToComponent` _returnvalue_3 (`self.FighterJetMesh`) "RightLauncher" "SnapToTarget" "SnapToTarget" "KeepRelative" true)
          (set `OreFiringComponent.EquippedWeapon` _returnvalue_3 (`self.BombingComponent`))
          (bind _returnvalue_4 (`|SpawnActorFromClass` "/Game/ProjectOre/Weapons/BP_SpacecraftLauncher.BP_SpacecraftLauncher_C" _returnvalue "Undefined" "OverrideRootScale" null null))
          (`/Engine/EditorBlueprintResources/StandardMacros.IsValid` _returnvalue_4
            (:`Is Valid`
              (`self.K2_AttachToComponent` _returnvalue_4 (`self.FighterJetMesh`) "LeftLauncher" "SnapToTarget" "SnapToTarget" "KeepRelative" true)
              (set `OreBombingComponent.EquippedWeapon2` _returnvalue_4 (`self.BombingComponent`)))))))))

(event `self.DropBomb_BP`
  (bind _returnvalue_x (`KismetMathLibrary.BreakVector` (`self.GetActorForwardVector`)))
  (bind _equippedweapon (`OreFiringComponent.EquippedWeapon` (`self.BombingComponent`)))
  (bind _equippedweapon2 (`OreBombingComponent.EquippedWeapon2` (`self.BombingComponent`)))
  (bind _velocity_x (`KismetMathLibrary.BreakVector` (`MovementComponent.Velocity` (`self.FloatingPawnMovement`))))
  (bind _returnvalue (* _velocity_x _returnvalue_x))
  (bind _returnvalue_2 (`SceneComponent.GetSocketTransform` (`OreWeapon.WeaponMesh` _equippedweapon2) "Muzzle" "RTS_World"))
  (bind _returnvalue_3 (`SceneComponent.GetSocketTransform` (`OreWeapon.WeaponMesh` _equippedweapon) "Muzzle" "RTS_World"))
  (if (`self.bCanFireMissileAgain`)
    (set `self.bCanFireMissileAgain` false)
    (`/Engine/EditorBlueprintResources/StandardMacros.FlipFlop`
      (:`A`
        (`|SpawnActorFromClass` "/Game/ProjectOre/Projectiles/BP_SpacecraftMissile.BP_SpacecraftMissile_C" _returnvalue_3 "Undefined" "OverrideRootScale" self _returnvalue self)
        (`GameplayStatics.PlaySoundAtLocation` (`OreWeapon.FireSound` _equippedweapon) (.location _returnvalue_3) (struct) 1.0 1.0 0.0 null null null)
        (`KismetSystemLibrary.K2_SetTimerDelegate` (delegate `AllowMissileFireAgain`) (`self.MissileFiringRate`)))
      (:`B`
        (`|SpawnActorFromClass` "/Game/ProjectOre/Projectiles/BP_SpacecraftMissile.BP_SpacecraftMissile_C" _returnvalue_2 "Undefined" "OverrideRootScale" self _returnvalue self)
        (`GameplayStatics.PlaySoundAtLocation` (`OreWeapon.FireSound` _equippedweapon2) (.location _returnvalue_2) (struct) 1.0 1.0 0.0 null null null)
        (`KismetSystemLibrary.K2_SetTimerDelegate` (delegate `AllowMissileFireAgain`) (`self.MissileFiringRate`))))))

(event `AllowMissileFireAgain`
  (set `self.bCanFireMissileAgain` true))

(fn `UserConstructionScript`)