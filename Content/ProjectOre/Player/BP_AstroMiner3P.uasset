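; Third-person astro miner character that spawns with a gun attached to its right arm and registered with its FiringComponent.
; Tick procedurally animates grounded walking with sine-driven limb swings and body/head wobble, holding the right arm raised when armed.
; Footstep audio is unmuted while walking and muted when stopped.
; A jump event splays arms and legs, mutes footsteps and plays the jump sound.
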(event `self.ReceiveBeginPlay`
  (`parent.ReceiveBeginPlay`)
  (`AudioComponent.SetVolumeMultiplier` (`self.FootStepSound`) 0.0)
  ;[0.9453 1 0] Automatically equip Gun (or Rifle)
  (bind _returnvalue (`|SpawnActorFromClass` "/Game/ProjectOre/Weapons/BP_Gun.BP_Gun_C" (`SceneComponent.K2_GetComponentToWorld` (`self.RightArm`)) "AlwaysSpawn" "OverrideRootScale" null null))
  (`/Engine/EditorBlueprintResources/StandardMacros.IsValid` _returnvalue
    (:`Is Valid`
      (`self.K2_AttachToComponent` _returnvalue (`self.RightArm`) "GunSocket" "SnapToTarget" "SnapToTarget" "KeepRelative" true)
      (set `OreFiringComponent.EquippedWeapon` _returnvalue (`self.FiringComponent`))
      (set `self.bArmed` true))))

(event `self.ReceiveTick`
  (params (DeltaSeconds :type "Float (single-precision)"))
  (bind _armrollangle (`self.ArmRollAngle`))
  (bind _charactermovement (`self.CharacterMovement`))
  (bind _bodypitchangle (`self.BodyPitchAngle`))
  (bind _legrollangle (`self.LegRollAngle`))
  (bind _legrollangle_2 (`self.LegRollAngle`))
  (bind _armrollangle_2 (`self.ArmRollAngle`))
  (bind _returnvalue (`KismetMathLibrary.MapRangeClamped` (`KismetMathLibrary.DegSin` (* (`self.ElapsedTime`) (`self.DegreesPerSec`))) 1.0 -1.0 0.0 1.0))
  (bind _returnvalue_2 (> (`KismetMathLibrary.VSize` (`MovementComponent.Velocity` _charactermovement)) 0.0))
  (bind _returnvalue_3 (`KismetMathLibrary.Lerp` _bodypitchangle (* _bodypitchangle -1.0) _returnvalue))
  (if (and (not (`NavMovementComponent.IsFalling` _charactermovement)) _returnvalue_2)
    (set `self.ElapsedTime` (+ DeltaSeconds (`self.ElapsedTime`)))
    ;[0 1 0.4141] Set the arm & legs joint rotations
    (`SceneComponent.K2_SetRelativeRotation` (`self.Joint_RightLegBP`) (`KismetMathLibrary.MakeRotator` (`KismetMathLibrary.Lerp` _legrollangle_2 (* _legrollangle_2 -1.0) _returnvalue)) false false)
    (`SceneComponent.K2_SetRelativeRotation` (`self.Joint_LeftLegBP`) (`KismetMathLibrary.MakeRotator` (`KismetMathLibrary.Lerp` (* _legrollangle -1.0) _legrollangle _returnvalue)) false false)
    (`SceneComponent.K2_SetRelativeRotation` (`self.Joint_LeftArmBP`) (`KismetMathLibrary.MakeRotator` (`KismetMathLibrary.Lerp` _armrollangle_2 (* _armrollangle_2 -1.0) _returnvalue)) false false)
    (`SceneComponent.K2_SetRelativeRotation` (`self.Joint_RightArmBP`) (`KismetMathLibrary.MakeRotator` (`KismetMathLibrary.SelectFloat` -75.0 (`KismetMathLibrary.Lerp` (* _armrollangle -1.0) _armrollangle _returnvalue) (`self.bArmed`))) false false)
    ;[0.2422 1 0] Wobble body and head
    (`SceneComponent.K2_SetRelativeRotation` (`self.Body2`) (`KismetMathLibrary.MakeRotator` 0.0 _returnvalue_3) false false)
    (`SceneComponent.K2_SetRelativeRotation` (`self.Head`) (`KismetMathLibrary.MakeRotator` 0.0 _returnvalue_3) false false)
    (`AudioComponent.SetVolumeMultiplier` (`self.FootStepSound`) 1.0)
    (elif (not _returnvalue_2)
      (`AudioComponent.SetVolumeMultiplier` (`self.FootStepSound`) 0.0)
      (`SceneComponent.K2_SetRelativeRotation` :`self` (`self.Joint_RightLegBP`))
      (`SceneComponent.K2_SetRelativeRotation` :`self` (`self.Joint_LeftLegBP`))
      (`SceneComponent.K2_SetRelativeRotation` :`self` (`self.Joint_LeftArmBP`))
      (`SceneComponent.K2_SetRelativeRotation` :`self` (`self.Body2`))
      (`SceneComponent.K2_SetRelativeRotation` :`self` (`self.Head`))
      ;[1 0.1875 0] Special case: are we armed or not?
      (if (not (`self.bArmed`))
        (`SceneComponent.K2_SetRelativeRotation` :`self` (`self.Joint_RightArmBP`))))))

(event `self.ExtendArmsLegsAtJump`
  (params (ArmRollDegrees :type "Float (single-precision)") (LegRollDegrees :type "Float (single-precision)"))
  (`SceneComponent.K2_SetRelativeRotation` (`self.Joint_RightArmBP`) (`KismetMathLibrary.MakeRotator` (* ArmRollDegrees -1.0)) false false)
  (`SceneComponent.K2_SetRelativeRotation` (`self.Joint_LeftArmBP`) (`KismetMathLibrary.MakeRotator` ArmRollDegrees) false false)
  (`SceneComponent.K2_SetRelativeRotation` (`self.Joint_RightLegBP`) (`KismetMathLibrary.MakeRotator` LegRollDegrees) false false)
  (`SceneComponent.K2_SetRelativeRotation` (`self.Joint_LeftLegBP`) (`KismetMathLibrary.MakeRotator` (* LegRollDegrees -1.0)) false false)
  (`AudioComponent.SetVolumeMultiplier` (`self.FootStepSound`) 0.0)
  (`GameplayStatics.PlaySoundAtLocation` "/Game/ProjectOre/Player/JumpSound.JumpSound" (`self.K2_GetActorLocation`) (struct) 1.0 1.0 0.1 null null null))

(fn `UserConstructionScript`)