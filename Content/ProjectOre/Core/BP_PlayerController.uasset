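; Player controller for Project Ore that handles toggling the pause menu through a PauseOreGame event.
; Pausing lazily creates and caches the WBP_PauseMenu widget, shows it, pauses the game, hides the game mode's main HUD and switches input to UI-only focused on the menu.
; Unpausing collapses the menu, resumes the game, restores the HUD and returns to game-only input, tracked by an InPauseMenu flag.
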(event `self.PauseOreGame`
  (if (`self.bInPauseMenu`)
    (`Widget.SetVisibility` (`self.PauseMenu`) "Collapsed")
    (`GameplayStatics.SetGamePaused` false)
    (`Widget.SetVisibility` (`OreGameMode.MainHUD` (`OreGameplayStatics.GetOreGameMode`)) "Visible")
    (set `self.bInPauseMenu` false)
    (`WidgetBlueprintLibrary.SetInputMode_GameOnly` self)
    (else
      (`/Engine/EditorBlueprintResources/StandardMacros.IsValid` (`self.PauseMenu`)
        (:`Is Valid`
          _)
        (:`Is Not Valid`
          (bind _returnvalue (`|CreateWidget` "/Game/ProjectOre/UI/WBP_PauseMenu.WBP_PauseMenu_C" self))
          (bind _output_get (set `self.PauseMenu` _returnvalue))
          (`UserWidget.AddToViewport` _output_get 0)))
      (`Widget.SetVisibility` (`self.PauseMenu`) "Visible")
      (`GameplayStatics.SetGamePaused` true)
      (`Widget.SetVisibility` (`OreGameMode.MainHUD` (`OreGameplayStatics.GetOreGameMode`)) "Collapsed")
      (set `self.bInPauseMenu` true)
      (`WidgetBlueprintLibrary.SetInputMode_UIOnlyEx` self (`self.PauseMenu`)))))

(fn `UserConstructionScript`)