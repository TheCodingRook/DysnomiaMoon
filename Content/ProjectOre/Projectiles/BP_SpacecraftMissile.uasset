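; Spacecraft missile projectile that explodes when it overlaps the landscape or a meteor, dealing full radial damage, playing an explosion sound and destroying itself.
; Both damage and sound are centered on the overlapped actor's location, not the missile's.
; The construction script adds ExtraSpeed to the base launch speed and builds the damage ignore list from all missile defences and ore pipelines, the third-person player character and the owner.
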(event `self.ReceiveActorBeginOverlap`
  (params (OtherActor :type "Actor Object Reference"))
  (bind _returnvalue (`self.K2_GetActorLocation` OtherActor))
  (cast `Landscape` OtherActor
    (:`then`
      _)
    (:`CastFailed`
      (cast `/Game/ProjectOre/LevelElements/BP_Meteor` OtherActor)))
  (`GameplayStatics.ApplyRadialDamage` 75.0 _returnvalue 200.0 null (`self.ActorsToIgnore`) (`self.GetOwner`) (`OreGameplayStatics.GetOrePlayerController`) true)
  (`GameplayStatics.PlaySoundAtLocation` "/Game/ProjectOre/Audio/A_Explosion.A_Explosion" _returnvalue (struct) 1.0 1.0 0.0 null null null)
  (`/Engine/EditorBlueprintResources/StandardMacros.IsValid` self
    (:`Is Valid`
      (`self.K2_DestroyActor`))))

(fn `UserConstructionScript`
  (bind _actorstoignore (`self.ActorsToIgnore`))
  (set `ProjectileMovementComponent.InitialSpeed` (+ 800.0 (`self.ExtraSpeed`)) (`self.ProjectileMovement`))
  (bind _outactors (`GameplayStatics.GetAllActorsOfClass` "/Game/ProjectOre/LevelElements/BP_MissileDefence.BP_MissileDefence_C"))
  (`KismetArrayLibrary.Array_Append` (`self.ActorsToIgnore`) _outactors)
  (bind _outactors_2 (`GameplayStatics.GetAllActorsOfClass` "/Script/Ore.OrePipeline"))
  (`KismetArrayLibrary.Array_Append` (`self.ActorsToIgnore`) _outactors_2)
  (`KismetArrayLibrary.Array_Add` _actorstoignore (`OreGameplayStatics.GetOreCharacter3P`))
  (`KismetArrayLibrary.Array_Add` _actorstoignore (`self.GetOwner`)))