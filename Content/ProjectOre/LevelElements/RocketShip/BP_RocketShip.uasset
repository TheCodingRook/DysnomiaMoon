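; Rocket ship level element that holds loaded fuel and gold and launches once it has enough fuel and either its timer elapses or its gold is full.
; While in launch position, Tick feeds countdown and supply ratios to the game mode's HUD.
; Launching, also exposed as EmergencyLaunch, adds a homing projectile movement component, broadcasts the launch and raises engine audio.
; Damage only decrements Health, and the velocity timeline is never triggered.
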(event `self.ReceiveBeginPlay`
  (bind _asbp_ore_game_mode (cast `/Game/ProjectOre/Core/BP_OreGameMode` (`OreGameplayStatics.GetOreGameMode`))
    (:`then`
      (set `self.TheGameMode` _asbp_ore_game_mode))
    (:`CastFailed`
      _))
  (`AudioComponent.SetVolumeMultiplier` (`self.Audio_RocketEngineLaunch_Cue`) 0.0)
  (add `self.OnTakeAnyDamage` (delegate `ReduceHealth`)))

(event `EmergencyLaunch`
  (`self.LaunchRocket` :!label _label)
  (`self.OnRocketHasLaunched`)
  (`/Engine/EditorBlueprintResources/StandardMacros.DoOnce` false :!label _label_2
    (:`Completed`
      (`AudioComponent.SetVolumeMultiplier` (`self.Audio_RocketEngineLaunch_Cue`) 0.75))))

(event `ReduceHealth` :!signature `self.OnTakeAnyDamage`
  (params (DamagedActor :type "Actor Object Reference") (Damage :type "Float (double-precision)") (DamageType :type "DamageType Object Reference") (InstigatedBy :type "Controller Object Reference") (DamageCauser :type "Actor Object Reference"))
  (set `self.Health` (- (`self.Health`) Damage)))

(event `self.ReceiveTick`
  (params (DeltaSeconds :type "Float (single-precision)"))
  (bind _thegamemode (`self.TheGameMode`))
  (bind _thegamemode_2 (`self.TheGameMode`))
  (bind _mainhud (`OreGameMode.MainHUD` _thegamemode_2))
  ;[0 0.625 1] Automatic launch on a timer
  (if (`self.bInLaunchPosition`)
    (`/Engine/EditorBlueprintResources/StandardMacros.IsValid` _thegamemode_2
      (:`Is Valid`
        (`OreHUD.UpdateRemainingTime` _mainhud (- (`self.LaunchEverySeconds`) (`self.ElapsedTime`)))
        (bind _output_get (set `self.ElapsedTime` (+ DeltaSeconds (`self.ElapsedTime`))))
        (`OreHUD.UpdateSupplies` _mainhud (/ (`self.LoadedFuel`) (`self.MinFuelRequired`)) (/ (`self.LoadedGold`) (`self.MaxGoldCapacity`)))
        (if (and (>= _output_get (`self.LaunchEverySeconds`)) (>= (`self.LoadedFuel`) (`self.MinFuelRequired`)))
          (set `self.ElapsedTime` 0.0 :!label _label_3)
          (goto _label)
          (elif (and (>= (`self.LoadedGold`) (`self.MaxGoldCapacity`)) (>= (`self.LoadedFuel`) (`self.MinFuelRequired`)))
            (goto _label_3)))))
    (else
      (`/Engine/EditorBlueprintResources/StandardMacros.IsValid` _thegamemode
        (:`Is Valid`
          (`OreHUD.UpdateRemainingTime` (`OreGameMode.MainHUD` _thegamemode) 0.0))))))

(event `Reset_DoOnce_SetVolume`
  (goto _label_2 :!via `Reset`))

(event `LaunchRocket`
  ;[0 0.8359 1] Launch sequence
  (set `self.bAirborne` true)
  (set `self.bInLaunchPosition` false)
  (bind _returnvalue (`AddComponent|NODE_AddProjectileMovementComponent-0`))
  (set `ProjectileMovementComponent.HomingTargetComponent` (`Actor.RootComponent` (`self.HomingTarget`)) _returnvalue)
  (`/Engine/EditorBlueprintResources/StandardMacros.DoOnce` false :!label _label_4))

(event `Reset_DoOnce_LaunchTimeline`
  ;[0 0.8359 1] Launch sequence
  (goto _label_4 :!via `Reset`))

(event `RemoveProjectileComponent`
  (bind _returnvalue (`self.GetComponentByClass` "/Script/Engine.ProjectileMovementComponent"))
  (if (`KismetSystemLibrary.IsValid` _returnvalue)
    (`ActorComponent.K2_DestroyComponent` _returnvalue)))

(fn `UserConstructionScript`)