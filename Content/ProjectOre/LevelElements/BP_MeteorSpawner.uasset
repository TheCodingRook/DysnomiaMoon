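; Volume actor that spawns meteors and also recycles any BP_RocketShip overlapping it back to launch.
; A looping timer, its interval fixed or randomized once at BeginPlay, spawns the actor class at random points in the volume with random rotation and scale.
; A DoOnce-gated overlap teleports the rocket to its reset position, clears its cargo, then raises it to launch position by timeline.
; Actor-pool spawning is present but unconnected.
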(event `self.ReceiveBeginPlay`
  (`KismetSystemLibrary.K2_SetTimerDelegate` (delegate `SpawnMeteor`) (`KismetMathLibrary.SelectFloat` (`self.SpawnFrequency`) (`KismetMathLibrary.RandomFloatInRange` (`self.MinSpawnDelay`) (`self.MaxSpawnDelay`)) (`self.bFixedFrequency`)) true))

(event `SpawnMeteor`
  (bind (_origin _boxextent) (`KismetSystemLibrary.GetComponentBounds` (`self.VolumeShape`)))
  ;[1 0 0.09375] Old - direct spawn - implementation
  (bind _returnvalue (`|SpawnActorFromClass` (`self.SpawnActorClass`) (`KismetMathLibrary.MakeTransform` (`KismetMathLibrary.RandomPointInBoundingBox` _origin _boxextent) (`KismetMathLibrary.RandomRotator` true) (`KismetMathLibrary.Conv_DoubleToVector` (`KismetMathLibrary.RandomFloatInRange` 0.75 1.25))) "Undefined" "OverrideRootScale" self null))
  (message `OreActorPoolInterface.SetupValues` _returnvalue))

(event `self.ReceiveTick`
  (params (DeltaSeconds :type "Float (single-precision)")))

(event `Reset_DoOnce`
  (bind (_launchposition_x _launchposition_y) (`KismetMathLibrary.BreakVector` (`self.LaunchPosition`)))
  (bind (_resetposition_x _resetposition_y _resetposition_z) (`KismetMathLibrary.BreakVector` (`self.ResetPosition`)))
  (bind (_launchposition_x_2 _launchposition_y_2 _launchposition_z) (`KismetMathLibrary.BreakVector` (`self.LaunchPosition`)))
  (bind _overlappedrocket (`self.OverlappedRocket`))
  (bind _overlappedrocket_2 (`self.OverlappedRocket`))
  (goto _label :!via `Reset`))

(event `self.ReceiveActorBeginOverlap`
  (params (OtherActor :type "Actor Object Reference"))
  (bind (_launchposition_x _launchposition_y) (`KismetMathLibrary.BreakVector` (`self.LaunchPosition`)))
  (bind (_resetposition_x _resetposition_y _resetposition_z) (`KismetMathLibrary.BreakVector` (`self.ResetPosition`)))
  (bind (_launchposition_x_2 _launchposition_y_2 _launchposition_z) (`KismetMathLibrary.BreakVector` (`self.LaunchPosition`)))
  (bind _overlappedrocket (`self.OverlappedRocket`))
  (bind _overlappedrocket_2 (`self.OverlappedRocket`))
  (bind _asbp_rocket_ship (cast `/Game/ProjectOre/LevelElements/RocketShip/BP_RocketShip` OtherActor))
  (`/Engine/EditorBlueprintResources/StandardMacros.DoOnce` false :!label _label
    (:`Completed`
      (bind _output_get (set `self.OverlappedRocket` _asbp_rocket_ship))
      (`/Game/ProjectOre/LevelElements/RocketShip/BP_RocketShip.RemoveProjectileComponent` _output_get)
      (`AudioComponent.SetVolumeMultiplier` (`/Game/ProjectOre/LevelElements/RocketShip/BP_RocketShip.Audio_RocketEngineLaunch_Cue` _output_get) 0.0)
      (`self.K2_SetActorLocation` (`self.OverlappedRocket`) (`self.ResetPosition`) false true)
      (set `/Game/ProjectOre/LevelElements/RocketShip/BP_RocketShip.bAirborne` false (`self.OverlappedRocket`))
      (set `RocketShipBase.LoadedGold` 0.0 _overlappedrocket_2)
      (set `RocketShipBase.LoadedFuel` 0.0 _overlappedrocket_2)
      (bind (_direction _alpha) (`Timeline|Timeline_0` :!via `PlayFromStart`)
        (:`Update`
          (`self.K2_SetActorLocation` (`self.OverlappedRocket`) (`KismetMathLibrary.MakeVector` _launchposition_x _launchposition_y (`KismetMathLibrary.Lerp` _resetposition_z _launchposition_z _alpha)) false false))
        (:`Finished`
          (set `RocketShipBase.bInLaunchPosition` true _overlappedrocket)
          (`/Game/ProjectOre/LevelElements/RocketShip/BP_RocketShip.Reset_DoOnce_LaunchTimeline` _overlappedrocket)
          (`/Game/ProjectOre/LevelElements/RocketShip/BP_RocketShip.Reset_DoOnce_SetVolume` _overlappedrocket)
          (`self.Reset_DoOnce`))))))

(fn `UserConstructionScript`)