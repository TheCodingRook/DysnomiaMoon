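; Missile defence building that fires homing missiles at meteors entering its range, provided it is powered, switched on and resourced.
; Overlapping meteors join a target list and trigger a launch, while a looping timer fires capped barrages from random tagged launchers.
; Infection turns it on friendly fighter jets through a repeating timer until cleared.
; Missiles are spawned directly; a pooled FireMissile function exists but is not called here.
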(event `Target Building`
  (bind _buildingtargets (`self.BuildingTargets`))
  (bind _returnvalue (`KismetArrayLibrary.Array_Length` _buildingtargets))
  ;[0.6406 0 1] Target our own buildings!
  (if (> _returnvalue 0)
    (`KismetArrayLibrary.Array_AddUnique` (`self.ActorTargets`) (`|GetArrayItem` _buildingtargets (`KismetMathLibrary.RandomInteger` _returnvalue)))))

(event `TargetSpacecraft`
  ;[0.7344 1 0] Target our own spacecraft!
  (bind _outactors (`GameplayStatics.GetAllActorsOfClass` "/Script/Ore.OreFighterJet"))
  (bind _returnvalue (`KismetArrayLibrary.Array_Length` _outactors))
  (if (> _returnvalue 0)
    (`KismetArrayLibrary.Array_AddUnique` (`self.ActorTargets`) (`|GetArrayItem` _outactors (`KismetMathLibrary.RandomInteger` _returnvalue)))))

(event `OreInfectionInterface.GetInfected`
  (bind _actortargets (`self.ActorTargets`))
  (bind _returnvalue (`KismetArrayLibrary.Array_Length` _actortargets))
  (bind _returnvalue_2 (`KismetMathLibrary.RandomInteger` _returnvalue))
  (`parent.GetInfected`)
  (`/Engine/EditorBlueprintResources/StandardMacros.DoOnce` false :!label _label
    (:`Completed`
      (`|ExecutionSequence`
        (:`then_0`
          (for _ (range 1)
            ;[0 1 0.2266] Remove a random meteor from the list of targets! except spacecraft or anything else of ours ;)
            (if (> _returnvalue 0)
              (cast `/Game/ProjectOre/LevelElements/BP_Meteor` (`|GetArrayItem` _actortargets _returnvalue_2))
              (`KismetArrayLibrary.Array_Remove` _actortargets _returnvalue_2))))
        (:`then_1`
          (`self.TargetSpacecraft`))
        (:`then_2`
          (bind _returnvalue_3 (`KismetSystemLibrary.K2_SetTimerDelegate` (delegate `TargetSpacecraft`) 60.0 true 60.0)) ; EVERY 60 SECONDS TARGET OUR SPACECRAFT AGAIN!
          (set `self.TargetSpacecraftTimer` _returnvalue_3))))))

(event `ResetInfectionGate`
  (`KismetSystemLibrary.K2_ClearAndInvalidateTimerHandle` (`self.TargetSpacecraftTimer`))
  (goto _label :!via `Reset`))

(event `self.ReceiveBeginPlay`
  (`parent.ReceiveBeginPlay`)
  (for _array_element (`self.GetComponentsByTag` "/Script/Engine.SceneComponent" "MissileLauncher")
    (`KismetArrayLibrary.Array_Add` (`self.MissileLaunchers`) _array_element)
    (`KismetSystemLibrary.K2_SetTimerDelegate` (delegate `LaunchBarrage`) 10.0 true)
    (bind _outactors (`GameplayStatics.GetAllActorsOfClass` "/Script/Ore.OreBuildingBase"))
    (bind _output_get (set `self.BuildingTargets` _outactors))
    (`KismetArrayLibrary.Array_RemoveItem` _output_get self)))

(event `self.ReceiveActorBeginOverlap`
  (params (OtherActor :type "Actor Object Reference"))
  (`parent.ReceiveActorBeginOverlap` OtherActor)
  (bind _asbp_meteor (cast `/Game/ProjectOre/LevelElements/BP_Meteor` OtherActor))
  (`KismetSystemLibrary.PrintString` (`KismetSystemLibrary.GetDisplayName` _asbp_meteor))
  (`KismetArrayLibrary.Array_AddUnique` (`self.ActorTargets`) _asbp_meteor)
  (add `self.OnActorBeginOverlap` _asbp_meteor (delegate `OnMeteorOverlapped`))
  ;[0.7109 0 1] Do we have the resources to operate?
  (bind _returnvalue (`self.CheckResources`))
  (if (and _returnvalue (`self.bPoweredOn`) (`self.bSwitchedOn`))
    (`self.LaunchMissile`)))

(event `self.DetectionSphere.OnComponentBeginOverlap`
  (params (OverlappedComponent :type "PrimitiveComponent Object Reference") (OtherActor :type "Actor Object Reference") (OtherComp :type "PrimitiveComponent Object Reference") (OtherBodyIndex :type Integer) (bFromSweep :type Boolean) (SweepResult :type "HitResult Structure (by ref)")))

(event `OnMeteorOverlapped` :!signature `self.OnActorBeginOverlap`
  (params (OverlappedActor :type "Actor Object Reference") (OtherActor :type "Actor Object Reference"))
  (cast `/Game/ProjectOre/Weapons/BP_Missile2` OtherActor)
  (`KismetArrayLibrary.Array_RemoveItem` (`self.ActorTargets`) (stale `self.ReceiveActorBeginOverlap` _asbp_meteor)))

(event `LaunchMissile`
  (bind _missilelaunchers (`self.MissileLaunchers`))
  (bind _output (`|GetArrayItem` (`self.ActorTargets`)))
  (`/Engine/EditorBlueprintResources/StandardMacros.IsValid` _output
    (:`Is Valid`
      (bind _returnvalue (`|SpawnActorFromClass` "/Game/ProjectOre/Weapons/BP_Missile2.BP_Missile2_C" (`SceneComponent.K2_GetComponentToWorld` (`|GetArrayItem` _missilelaunchers (`KismetMathLibrary.RandomInteger` (`KismetArrayLibrary.Array_Length` _missilelaunchers)))) "AlwaysSpawn" "OverrideRootScale" (stale `self.ReceiveActorBeginOverlap` _asbp_meteor) null))
      (set `/Game/ProjectOre/Weapons/BP_Missile2.MyTarget` _output _returnvalue)
      (set `/Game/ProjectOre/Weapons/BP_Missile2.bValidHomingTarget` true _returnvalue)
      (`KismetArrayLibrary.Array_RemoveItem` (`self.ActorTargets`) _output))))

(event `OreInfectionInterface.OnInfectionCleared`
  (`parent.OnInfectionCleared`)
  (`KismetSystemLibrary.K2_ClearAndInvalidateTimerHandle` (`self.TargetSpacecraftTimer`))
  (`self.ResetInfectionGate`)
  ;[0.7109 0 1] Do we have the resources to operate?
  (bind _returnvalue (`self.CheckResources`))
  (if (and _returnvalue (`self.bPoweredOn`) (`self.bSwitchedOn`))
    (`self.LaunchBarrage`)))

(event `LaunchBarrage`
  (bind _missilelaunchers (`self.MissileLaunchers`))
  (bind _actortargets (`self.ActorTargets`))
  ;[0.7109 0 1] Do we have the resources to operate?
  (bind _returnvalue (`self.CheckResources`))
  (if (and _returnvalue (`self.bPoweredOn`) (`self.bSwitchedOn`))
    (for (_array_element _array_index) _actortargets
      (`/Engine/EditorBlueprintResources/StandardMacros.IsValid` _array_element
        (:`Is Not Valid`
          (`KismetArrayLibrary.Array_Remove` _actortargets _array_index))))
    (for (_array_element_2 _array_index_2) (`self.ActorTargets`)
      ;[1 0.6094 0] Break after 8 targets
      (if (> _array_index_2 7)
        (break)
        (else
          (bind _returnvalue_2 (`|SpawnActorFromClass` "/Game/ProjectOre/Weapons/BP_Missile2.BP_Missile2_C" (`SceneComponent.K2_GetComponentToWorld` (`|GetArrayItem` _missilelaunchers (`KismetMathLibrary.RandomInteger` (`KismetArrayLibrary.Array_Length` _missilelaunchers)))) "AlwaysSpawn" "OverrideRootScale" _array_element_2 null))
          (bind _output_get (set `/Game/ProjectOre/Weapons/BP_Missile2.MyTarget` _array_element_2 _returnvalue_2))
          (set `/Game/ProjectOre/Weapons/BP_Missile2.bValidHomingTarget` true _returnvalue_2)
          ;[0 0.1094 1] If we targeted one of our own stuff, just do it once!
          (cast `OreFighterJet` _output_get
            (:`then`
              (`KismetArrayLibrary.Array_RemoveItem` (`self.ActorTargets`) _array_element_2))
            (:`CastFailed`
              (bind _asore_building_base (cast `OreBuildingBase` _output_get))
              (`KismetArrayLibrary.Array_RemoveItem` (`self.BuildingTargets`) _asore_building_base))))))))

(fn `FireMissile`
  (returns (OutMissile :type "/Game/ProjectOre/Weapons/BP_Missile_Homing Object Reference"))
  (bind _returnvalue (`OreActorPoolComponent.RemoveFromPool` (`self.MissilesPool`)))
  (bind _asbp_missile_homing (cast `/Game/ProjectOre/Weapons/BP_Missile_Homing` _returnvalue))
  (return _asbp_missile_homing))

(fn `UserConstructionScript`
  (`parent.UserConstructionScript`))