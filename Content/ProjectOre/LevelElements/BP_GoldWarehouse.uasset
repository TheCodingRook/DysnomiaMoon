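; Gold warehouse level element tied to a rocket ship, with infection, tick and begin-play events deferring to its parent class.
; On BeginPlay it binds to the rocket's launch event, but that handler is empty.
; A disconnected, never-run graph holds logic to transfer gold and fuel from its resources into a rocket in launch position, rate-limited per second and capped by gold capacity and required fuel.
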(event `OreInfectionInterface.GetInfected`
  (`parent.GetInfected`))

(event `OreInfectionInterface.OnInfectionCleared`
  (`parent.OnInfectionCleared`))

(event `self.ReceiveTick`
  (params (DeltaSeconds :type "Float (single-precision)"))
  (`parent.ReceiveTick` DeltaSeconds))

(event `self.ReceiveBeginPlay`
  (bind _rocketship_bp (`self.RocketShip_BP`))
  (`parent.ReceiveBeginPlay`)
  (`/Engine/EditorBlueprintResources/StandardMacros.IsValid` _rocketship_bp
    (:`Is Valid`
      (add `/Game/ProjectOre/LevelElements/RocketShip/BP_RocketShip.OnRocketHasLaunched` _rocketship_bp (delegate `RocketLaunchedEvent`)))))

(event `RocketLaunchedEvent`)

(fn `UserConstructionScript`)