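; BP_InfectionManager is a level actor that periodically infects a random ore mine.
; Two seconds after BeginPlay it gathers all OreMineBase actors and randomizes the first interval.
; Tick accumulates time; when the interval elapses, it picks a mine, rerolls the timer and sends GetInfectedMessage if that mine is uninfected.
; For explosives and fuel mines, it also shows a HUD warning and increments the infection counter.
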(event `PickRandomInterval`
  (set `self.TimeUntilNextInfection` (`KismetMathLibrary.RandomFloatInRange` 20.0 120.0)))

(event `self.ReceiveBeginPlay`
  (`KismetSystemLibrary.Delay` 2.0)
  ;[0.1484 0 1] Find all the mines on this moon (except for gold - for now)
  (bind _outactors (`GameplayStatics.GetAllActorsOfClass` "/Script/Ore.OreMineBase"))
  (for _array_element _outactors
    (`KismetArrayLibrary.Array_Add` (`self.OreMines`) _array_element)
    (`self.PickRandomInterval`)))

(event `self.ReceiveTick`
  (params (DeltaSeconds :type "Float (single-precision)"))
  (bind _oremines (`self.OreMines`))
  (bind _chosenmine (`self.ChosenMine`))
  (set `self.ElapsedTime` (+ DeltaSeconds (`self.ElapsedTime`)))
  (if (>= (`self.ElapsedTime`) (`self.TimeUntilNextInfection`))
    (bind _output_get (set `self.ChosenMine` (`|GetArrayItem` _oremines (`KismetMathLibrary.RandomInteger` (`KismetArrayLibrary.Array_Length` _oremines)))))
    (set `self.ElapsedTime` 0.0)
    (`self.PickRandomInterval`)
    (if (not (`OreMineBase.bInfected` _output_get))
      (message `OreInfectionInterface.GetInfected` _output_get)
      (cast `/Game/ProjectOre/LevelElements/BP_ExplosivesMine` _chosenmine
        (:`then`
          (`OreHUD.GiveInfectionWarning` (`OreGameMode.MainHUD` (`OreGameplayStatics.GetOreGameMode`)) "Explosives"))
        (:`CastFailed`
          (cast `/Game/ProjectOre/LevelElements/BP_FuelMine` _chosenmine)
          (`OreHUD.GiveInfectionWarning` (`OreGameMode.MainHUD` (`OreGameplayStatics.GetOreGameMode`)) "Fuel")))
      (bind _aswbp_main_hud (cast `/Game/ProjectOre/UI/WBP_MainHUD` (`OreGameMode.MainHUD` (`OreGameplayStatics.GetOreGameMode`))))
      (`/Game/ProjectOre/UI/WBP_MainHUD.UpdateInfectionsCounter` _aswbp_main_hud 1))))

(fn `UserConstructionScript`)