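; BP_RocketTriggerVolume is a trigger volume that registers a rocket ship's cargo as shipped when the rocket overlaps it.
; On overlap with a BP_RocketShip, it adds the ship's loaded gold and parasites to the game mode's shipped totals and refreshes the main HUD counters.
; When shipped parasites reach three times the ship's max gold capacity, it pauses the game and shows the parasite game-over reason.
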(event `self.ReceiveActorBeginOverlap`
  (params (OtherActor :type "Actor Object Reference"))
  (bind _returnvalue (`OreGameplayStatics.GetOreGameMode`))
  (bind _returnvalue_2 (`OreGameplayStatics.GetOreGameMode`))
  (bind _mainhud (`OreGameMode.MainHUD` _returnvalue))
  (bind _asbp_rocket_ship (cast `/Game/ProjectOre/LevelElements/RocketShip/BP_RocketShip` OtherActor))
  (`|ExecutionSequence`
    (:`then_0`
      (set `OreGameMode.GoldShipped` (+ (`OreGameMode.GoldShipped` _returnvalue_2) (`RocketShipBase.LoadedGold` _asbp_rocket_ship)) _returnvalue_2)
      (`OreHUD.UpdateGoldShipped` (`OreGameMode.MainHUD` _returnvalue_2)))
    (:`then_1`
      (set `OreGameMode.ParasiteShipped` (+ (`OreGameMode.ParasiteShipped` _returnvalue) (`RocketShipBase.LoadedParasite` _asbp_rocket_ship)) _returnvalue)
      (`OreHUD.UpdateParasiteShipped` _mainhud)
      (if (>= (`OreGameMode.ParasiteShipped` _returnvalue) (* 3 (`RocketShipBase.MaxGoldCapacity` _asbp_rocket_ship)))
        (`GameplayStatics.SetGamePaused` true)
        (`OreHUD.DisplayWhyGameOver` _mainhud "Parasite")))))

(fn `UserConstructionScript`)