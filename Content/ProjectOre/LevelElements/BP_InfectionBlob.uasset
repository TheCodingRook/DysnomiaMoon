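; Destructible infection blob that loses health from any damage and plays a bullet impact sound at its location on each hit.
; When health runs out, it casts its owner to InfectionSpawnVolume, decrements that volume's spawn count and destroys itself.
; Destruction depends on that cast, so a blob without such an owner stays in the level at zero health.
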(event `self.ReceiveAnyDamage`
  (params (Damage :type "Float (single-precision)") (DamageType :type "DamageType Object Reference") (InstigatedBy :type "Controller Object Reference") (DamageCauser :type "Actor Object Reference"))
  (set `self.Health` (- (`self.Health`) Damage))
  (`GameplayStatics.PlaySoundAtLocation` "/Game/ProjectOre/Weapons/A_BulletImpact_Cue.A_BulletImpact_Cue" (`self.K2_GetActorLocation`) (struct) 1.0 1.0 0.0 null null null)
  (if (<= (`self.Health`) 0.0)
    (bind _asinfection_spawn_volume (cast `InfectionSpawnVolume` (`self.GetOwner`)))
    (`/Engine/EditorBlueprintResources/StandardMacros.DecrementInt` (`InfectionSpawnVolume.SpawnCount` _asinfection_spawn_volume)
      (:`  `
        (`self.K2_DestroyActor`)))))

(fn `UserConstructionScript`)