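; BP_Infrastructure is a switchable, infectable level element that shows its state through blinking indicator lights.
; BeginPlay gives meshes tagged "Lightbulb" dynamic materials, and Tick toggles their emissive switch while powered, keeping them dark otherwise.
; Infection turns the lights red and triples the blink speed once until cleared, which restores green and slows blinking.
; Switch toggles show amber when off; when on, emissive color follows infection but base color is always green.
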(event `self.ReceiveBeginPlay`
  ;[1 0.6094 0] Add all the lights here
  (for _array_element (`self.GetComponentsByTag` "/Script/Engine.StaticMeshComponent" "Lightbulb")
    (`PrimitiveComponent.CreateDynamicMaterialInstance` _array_element 0 "/Game/ProjectOre/LevelElements/MI_GreenLight.MI_GreenLight" "None")
    (`KismetArrayLibrary.Array_Add` (`self.Lights`) _array_element)))

(event `self.ReceiveTick`
  (params (DeltaSeconds :type "Float (single-precision)"))
  (if (`self.bPoweredOn`)
    (bind _output_get (set `self.TimeSinceLastToggle` (+ DeltaSeconds (`self.TimeSinceLastToggle`))))
    (if (>= _output_get (`self.BlinkingRate`))
      (for _array_element (`self.Lights`) :!label _label
        (bind _asmaterial_instance_dynamic (cast `MaterialInstanceDynamic` (`PrimitiveComponent.GetMaterial` _array_element 0)))
        (`MaterialInstanceDynamic.SetScalarParameterValue` _asmaterial_instance_dynamic "LightSwitch" (`self.EmissiveValue`)))
      (if (`self.bPoweredOn`)
        (set `self.TimeSinceLastToggle` 0.0)
        (`/Engine/EditorBlueprintResources/StandardMacros.FlipFlop`
          (:`A`
            (set `self.EmissiveValue` 0.0))
          (:`B`
            (set `self.EmissiveValue` 1.0)))))
    (else
      (set `self.EmissiveValue` 0.0)
      (set `self.TimeSinceLastToggle` 0.0)
      (goto _label))))

(event `OreInfectionInterface.GetInfected`
  (`parent.GetInfected`)
  (`/Engine/EditorBlueprintResources/StandardMacros.DoOnce` false :!label _label_2
    (:`Completed`
      (for _array_element (`self.Lights`)
        (bind _asmaterial_instance_dynamic (cast `MaterialInstanceDynamic` (`PrimitiveComponent.GetMaterial` _array_element 0)))
        (`MaterialInstanceDynamic.SetVectorParameterValue` _asmaterial_instance_dynamic "BaseColor" (`KismetMathLibrary.Conv_VectorToLinearColor` (`self.BaseColor_Red`)))
        (`MaterialInstanceDynamic.SetVectorParameterValue` _asmaterial_instance_dynamic "EmissiveColor" (`KismetMathLibrary.Conv_VectorToLinearColor` (`self.EmissiveColor_Red`))))
      (set `self.BlinkingRate` (/ (`self.BlinkingRate`) 3.0)))))

(event `OreInfectionInterface.OnInfectionCleared`
  (`parent.OnInfectionCleared`)
  (for _array_element (`self.Lights`)
    (bind _asmaterial_instance_dynamic (cast `MaterialInstanceDynamic` (`PrimitiveComponent.GetMaterial` _array_element 0)))
    (`MaterialInstanceDynamic.SetVectorParameterValue` _asmaterial_instance_dynamic "BaseColor" (`KismetMathLibrary.Conv_VectorToLinearColor` (`self.BaseColor_Green`)))
    (`MaterialInstanceDynamic.SetVectorParameterValue` _asmaterial_instance_dynamic "EmissiveColor" (`KismetMathLibrary.Conv_VectorToLinearColor` (`self.EmissiveColor_Green`)))
    (set `self.TimeSinceLastToggle` 0.0)
    (goto _label_2 :!via `Reset`))
  (set `self.BlinkingRate` (* (`self.BlinkingRate`) 3.0)))

(event `self.OnSwitchToggled`
  (params (InSwitchState :type Boolean))
  (bind _bswitchedon (`self.bSwitchedOn`))
  (`parent.OnSwitchToggled` InSwitchState)
  (for _array_element (`self.Lights`)
    (bind _asmaterial_instance_dynamic (cast `MaterialInstanceDynamic` (`PrimitiveComponent.GetMaterial` _array_element 0)))
    (`MaterialInstanceDynamic.SetVectorParameterValue` _asmaterial_instance_dynamic "BaseColor" (`KismetMathLibrary.Conv_VectorToLinearColor` (`KismetMathLibrary.SelectVector` (`KismetMathLibrary.SelectVector` (`self.BaseColor_Red`) (`self.BaseColor_Green`)) (`self.BaseColor_Amber`) _bswitchedon)))
    (`MaterialInstanceDynamic.SetVectorParameterValue` _asmaterial_instance_dynamic "EmissiveColor" (`KismetMathLibrary.Conv_VectorToLinearColor` (`KismetMathLibrary.SelectVector` (`KismetMathLibrary.SelectVector` (`self.EmissiveColor_Red`) (`self.EmissiveColor_Green`) (`self.bInfected`)) (`self.EmissiveColor_Amber`) _bswitchedon)))))

(fn `UserConstructionScript`)