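; Switchable pipeline that carries pooled ore lumps along a spline and delivers them to an Offtaker building, spreading infection to it.
; While switched on, Tick spawns a lump each FlowRate interval, advances lumps one spline point per interval by lerping, and returns arrivals to the pool.
; Helper functions rebuild the spline from tagged instanced-mesh pipe sections and add or remove end pipes.
; Toggling the switch recolours the light bulb's emissive material.
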(event `self.ReceiveBeginPlay`
  (`PrimitiveComponent.CreateDynamicMaterialInstance` (`self.LightBulb`) 0 "/Game/ProjectOre/LevelElements/M_GreenLight.M_GreenLight" "None"))

(event `self.ReceiveTick`
  (params (DeltaSeconds :type "Float (single-precision)"))
  (bind _offtaker (`self.Offtaker`))
  (bind _returnvalue_location (`KismetMathLibrary.BreakTransform` (`SplineComponent.GetTransformAtSplinePoint` (`self.SplineComponent`) 0 "World" false)))
  (bind _returnvalue_location_2 (`KismetMathLibrary.BreakTransform` (`SplineComponent.GetTransformAtSplinePoint` (`self.SplineComponent`) 0 "World" false)))
  (if (`self.bSwitchedOn`)
    (bind _output_get (set `self.ElapsedTime` (+ DeltaSeconds (`self.ElapsedTime`))))
    (bind _remainder (`KismetMathLibrary.FMod` _output_get (`self.FlowRate`)))
    ;[0 1 0.7656] Is it time to spawn a new lump?
    (if (and (< _remainder (`self.PreviousRemainder`)) (`self.bSpawnNewLump`))
      ;[0.2187 1 0] If so...
      ;;[0.9453 0 1] Increase every lump's index position on the spline
      (for _array_element (`self.MovingOreLumps`)
        (`/Engine/EditorBlueprintResources/StandardMacros.IncrementInt` (`MovingOreLump.CurrentSplineIndex` _array_element)))
      ;;[0 0.2031 1] Spawn a new lump
      (bind _returnvalue (`OreActorPoolComponent.RemoveFromPool` (`self.OreActorPool`)))
      ;;[0 0.4141 1] Infect if necessary
      (if (`self.bInfected`)
        (message `OreInfectionInterface.GetInfected` _returnvalue))
      (bind _asmoving_ore_lump (cast `MovingOreLump` _returnvalue))
      (`self.K2_SetActorLocation` _returnvalue _returnvalue_location_2 false true)
      (`KismetArrayLibrary.Array_AddUnique` (`self.MovingOreLumps`) _asmoving_ore_lump)
      (set `MovingOreLump.OriginLocation` _returnvalue_location _asmoving_ore_lump)
      (set `self.bSpawnNewLump` false)
      (else
        (set `self.bSpawnNewLump` true) ; Reset the flag for next time we can spawn
      ))
    (set `self.PreviousRemainder` _remainder)
    ;[0 0.5312 1] Check to see if the lump of ore has reached the end of the pipeline...
    (for (_array_element_2 _array_index) (`self.MovingOreLumps`)
      (if (and (== (`MovingOreLump.CurrentSplineIndex` _array_element_2) (- (`SplineComponent.GetNumberOfSplinePoints` (`self.SplineComponent`)) 1)) (`KismetMathLibrary.NearlyEqual_FloatFloat` (`KismetMathLibrary.Vector_Distance` (`self.K2_GetActorLocation` _array_element_2) (`MovingOreLump.TargetLocation` _array_element_2)) 0.0 0.01))
        ;[0 1 0.8359] ... if so, process the ore lump into the offtaker building
        (`/Engine/EditorBlueprintResources/StandardMacros.IsValid` _offtaker
          (:`Is Valid`
            (`OreBuildingBase.AcceptResourceFromPipeline` _offtaker (`OreLumpBase.OreType` _array_element_2) (`OreLumpBase.QuantityPerLump` _array_element_2)))
          (:`Is Not Valid`
            _))
        (if (`OreLumpBase.IsInfected` _array_element_2)
          (`OreInfectionInterface.GetInfected` _offtaker)
          (message `OreInfectionInterface.OnInfectionCleared` _array_element_2) ; After infecting building, this lump can go back in the ActorPool as 'clean'
        )
        (`OreActorPoolComponent.ReturnToPool` (`self.OreActorPool`) _array_element_2)
        (`KismetArrayLibrary.Array_Remove` (`self.MovingOreLumps`) _array_index)))
    ;[1 0 0.7031] Move each lump in the array along the spline!
    (for _array_element_3 (`self.MovingOreLumps`)
      (bind _currentsplineindex (`MovingOreLump.CurrentSplineIndex` _array_element_3))
      (bind _returnvalue_location_3 (`KismetMathLibrary.BreakTransform` (`SplineComponent.GetTransformAtSplinePoint` (`self.SplineComponent`) (`KismetMathLibrary.Clamp` _currentsplineindex 0 (- (`SplineComponent.GetNumberOfSplinePoints` (`self.SplineComponent`)) 1)) "World" false)))
      (set `MovingOreLump.OriginLocation` _returnvalue_location_3 _array_element_3)
      (bind _returnvalue_location_4 (`KismetMathLibrary.BreakTransform` (`SplineComponent.GetTransformAtSplinePoint` (`self.SplineComponent`) (`KismetMathLibrary.Clamp` (+ _currentsplineindex 1) 0 (- (`SplineComponent.GetNumberOfSplinePoints` (`self.SplineComponent`)) 1)) "World" false)))
      (set `MovingOreLump.TargetLocation` _returnvalue_location_4 _array_element_3)
      (`self.K2_SetActorLocation` _array_element_3 (`KismetMathLibrary.VLerp` (`MovingOreLump.OriginLocation` _array_element_3) (`MovingOreLump.TargetLocation` _array_element_3) (`KismetMathLibrary.FClamp` (/ _remainder (`self.FlowRate`)))) false false))))

(event `self.OnSwitchToggled`
  (params (InSwitchState :type Boolean))
  (`parent.OnSwitchToggled` InSwitchState)
  (bind _asmaterial_instance_dynamic (cast `MaterialInstanceDynamic` (`PrimitiveComponent.GetMaterial` (`self.LightBulb`) 0)))
  (`MaterialInstanceDynamic.SetVectorParameterValue` _asmaterial_instance_dynamic "EmissiveColor" (`KismetMathLibrary.Conv_VectorToLinearColor` (`KismetMathLibrary.SelectVector` (`self.EmmissiveColorGreen`) (`self.EmissiveColorRed`) (`self.bSwitchedOn`)))))

(fn `AddPipe`
  (locals (LastValidIndex :type Integer))
  (bind _instancedmeshes (`self.InstancedMeshes`))
  (bind _output (`|GetArrayItem` _instancedmeshes (`KismetArrayLibrary.Array_LastIndex` _instancedmeshes)))
  (bind _returnvalue (`InstancedStaticMeshComponent.GetInstanceCount` _output))
  (if (> _returnvalue 0)
    (`InstancedStaticMeshComponent.AddInstance` _output (`KismetMathLibrary.ComposeTransforms` (`self.TransformOffset`) (`InstancedStaticMeshComponent.GetInstanceTransform` _output (- _returnvalue 1) false)))))

(fn `AddSplinePoint`
  (params (InLocation :type "Vector Structure"))
  (`SplineComponent.AddSplinePoint` (`self.SplineComponent`) InLocation "Local" true))

(fn `AddSplinePointsInMeshes`
  (params (InInstancedMesh :type "InstancedStaticMeshComponent Object Reference"))
  (for _index (range (`InstancedStaticMeshComponent.GetInstanceCount` InInstancedMesh))
    (`self.AddSplinePoint` (`KismetMathLibrary.MakeVector` (.x (+ (.location (`InstancedStaticMeshComponent.GetInstanceTransform` InInstancedMesh _index false)) (`SceneComponent.RelativeLocation` InInstancedMesh))) (.y (+ (.location (`InstancedStaticMeshComponent.GetInstanceTransform` InInstancedMesh _index false)) (`SceneComponent.RelativeLocation` InInstancedMesh))) (+ (.z (+ (.location (`InstancedStaticMeshComponent.GetInstanceTransform` InInstancedMesh _index false)) (`SceneComponent.RelativeLocation` InInstancedMesh))) 15.0)))))

(fn `RefreshPipeSections`
  (`SplineComponent.ClearSplinePoints` (`self.SplineComponent`) true)
  (`KismetArrayLibrary.Array_Clear` (`self.InstancedMeshes`))
  (for _array_element (`self.ComponentOrder`)
    (bind _returnvalue (`self.GetComponentsByTag` "/Script/Engine.InstancedStaticMeshComponent" _array_element))
    (if (`KismetArrayLibrary.Array_IsValidIndex` _returnvalue)
      (bind _output (`|GetArrayItem` _returnvalue))
      (`KismetArrayLibrary.Array_AddUnique` (`self.InstancedMeshes`) _output)
      (`self.AddSplinePointsInMeshes` _output)
      (`KismetSystemLibrary.PrintString` (`KismetSystemLibrary.GetDisplayName` _output)))))

(fn `RemovePipe`
  (bind _instancedmeshes (`self.InstancedMeshes`))
  (bind _output (`|GetArrayItem` _instancedmeshes (`KismetArrayLibrary.Array_LastIndex` _instancedmeshes)))
  (bind _returnvalue (`InstancedStaticMeshComponent.GetInstanceCount` _output))
  (if (> _returnvalue 0)
    (`KismetSystemLibrary.PrintString` (`KismetStringLibrary.Conv_IntToString` _returnvalue))
    (`InstancedStaticMeshComponent.RemoveInstance` _output (- _returnvalue 1))))

(fn `UserConstructionScript`)