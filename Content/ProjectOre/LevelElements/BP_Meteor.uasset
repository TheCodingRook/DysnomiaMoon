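; BP_Meteor is a falling hazard actor that heavily damages whatever it overlaps and can be destroyed by BP_Missile2.
; Overlapping landscape, pipelines or buildings other than missile defences notifies OreGameMode of a crash, then destroys the meteor after a short delay.
; A mesh hit on landscape adds a world camera shake before the same crash path.
; Logic returning it to the spawner's actor pool is unconnected.
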(event `self.ReceiveActorBeginOverlap`
  (params (OtherActor :type "Actor Object Reference"))
  (`GameplayStatics.ApplyDamage` OtherActor 1000.0)
  (bind _asbp_missile_2 (cast `/Game/ProjectOre/Weapons/BP_Missile2` OtherActor)
    (:`then`
      (`KismetSystemLibrary.PrintString` (`KismetTextLibrary.Conv_TextToString` (`|FormatText` "{Name} was destroyed by {Missile}" (`KismetSystemLibrary.GetObjectName` self) (`KismetSystemLibrary.GetDisplayName` _asbp_missile_2)))))
    (:`CastFailed`
      (cast `Landscape` OtherActor
        (:`then`
          _)
        (:`CastFailed`
          (cast `OrePipeline` OtherActor
            (:`then`
              _)
            (:`CastFailed`
              (cast `OreBuildingBase` OtherActor)
              (cast `/Game/ProjectOre/LevelElements/BP_MissileDefence` OtherActor
                (:`CastFailed`
                  _))))))
      (bind _asore_game_mode (cast `OreGameMode` (`GameplayStatics.GetGameMode`) :!label _label))
      (`OreGameMode.OnMeteorCrashed` _asore_game_mode)))
  (`KismetSystemLibrary.Delay` 0.1)
  (`/Engine/EditorBlueprintResources/StandardMacros.IsValid` self
    (:`Is Valid`
      (`self.K2_DestroyActor`))))

(event `self.MeteorMesh.OnComponentHit`
  (params (HitComponent :type "PrimitiveComponent Object Reference") (OtherActor :type "Actor Object Reference") (OtherComp :type "PrimitiveComponent Object Reference") (NormalImpulse :type "Vector Structure") (Hit :type "HitResult Structure (by ref)"))
  (cast `Landscape` OtherActor)
  (`GameplayStatics.PlayWorldCameraShake` "/Game/ProjectOre/LevelElements/BP_OreCameraShake.BP_OreCameraShake_C" Hit_Location 0.0 5000.0 100.0 true)
  (goto _label))

(fn `UserConstructionScript`)